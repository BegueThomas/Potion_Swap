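; BP_LightCards_A is a light card prop that pairs a spot light with a plane mesh, configured per instance.
; The construction script pushes exposed intensity, temperature, indirect intensity, color and light function material values to the spot light.
; It applies the same three lighting channel toggles to both the light and SMPlaneA.
; The event graph holds only disabled stubs, so the script has no runtime logic.
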(fn `UserConstructionScript`
  (bind _spotlight (`self.SpotLight`))
  (bind _lightchannel0_on (`self.LightChannel0_ON`))
  (bind _lightchannel1_on (`self.LightChannel1_ON`))
  (bind _lightchannel2_on (`self.LightChannel2_ON`))
  (`LightComponent.SetIntensity` _spotlight (`self.Light Intensity`))
  (`LightComponent.SetTemperature` _spotlight (`self.Temperature`))
  (`LightComponent.SetIndirectLightingIntensity` _spotlight (`self.Indirect Intensity`))
  (`LightComponent.SetLightFunctionMaterial` _spotlight (`self.Light Function Material`))
  (`LightComponent.SetLightingChannels` _spotlight _lightchannel0_on _lightchannel1_on _lightchannel2_on)
  (`PrimitiveComponent.SetLightingChannels` (`self.SM_Plane_A`) _lightchannel0_on _lightchannel1_on _lightchannel2_on)
  (`LightComponent.SetLightColor` (`self.SpotLight`) (`KismetMathLibrary.Conv_ColorToLinearColor` (`self.Color`)) true))