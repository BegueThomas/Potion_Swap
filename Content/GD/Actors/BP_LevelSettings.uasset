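; BP_LevelSettings is an actor that sets which player forms (Blue, Red, Green) are locked in a level and which form the player starts in.
; On BeginPlay it caches BP_ThirdPersonGameMode, then uses that game mode's player reference to copy its lock flags onto the player.
; It then calls ChangeForm on the player with the configured first form.
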(event `Lock_Forms`
  (bind _player_ref (`/Game/GD/ThirdPerson/Blueprints/BP_ThirdPersonGameMode.Player_Ref` (stale `self.ReceiveBeginPlay` _output_get)))
  (set `/Game/GD/ThirdPerson/Blueprints/BP_ThirdPersonCharacter.Blue_Lock?` (`self.B_Lock`) _player_ref)
  (set `/Game/GD/ThirdPerson/Blueprints/BP_ThirdPersonCharacter.Red_lock?` (`self.R_Lock`) _player_ref)
  (set `/Game/GD/ThirdPerson/Blueprints/BP_ThirdPersonCharacter.Green_Lock?` (`self.G_Lock`) _player_ref))

(event `self.ReceiveBeginPlay`
  (bind _asbp_third_person_game_mode (cast `/Game/GD/ThirdPerson/Blueprints/BP_ThirdPersonGameMode` (`GameplayStatics.GetGameMode`)))
  (bind _output_get (set `self.Gamemode_Ref` _asbp_third_person_game_mode))
  (`self.Lock_Forms`)
  (`/Game/GD/ThirdPerson/Blueprints/BP_ThirdPersonCharacter.Change_Form` (`/Game/GD/ThirdPerson/Blueprints/BP_ThirdPersonGameMode.Player_Ref` _output_get) 0.0 (`self.First_Form`)))

(fn `UserConstructionScript`)