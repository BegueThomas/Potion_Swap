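; BP_Checkpoint is a checkpoint actor that updates the player's respawn point when reached.
; On BeginPlay it caches BP_ThirdPersonGameMode, then uses its stored character reference to filter overlaps on the Box trigger.
; The first valid overlap, gated by DoOnce, writes the checkpoint's location to the game mode's RespawnPoint and smoothly raises Cube1 with MoveComponentTo as visual feedback.
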(event `self.ReceiveBeginPlay`
  (bind _asbp_third_person_game_mode (cast `/Game/GD/ThirdPerson/Blueprints/BP_ThirdPersonGameMode` (`GameplayStatics.GetGameMode`)))
  (set `self.As BP Third Person Game Mode` _asbp_third_person_game_mode))

(event `self.Box.OnComponentBeginOverlap`
  (params (OverlappedComponent :type "PrimitiveComponent Object Reference") (OtherActor :type "Actor Object Reference") (OtherComp :type "PrimitiveComponent Object Reference") (OtherBodyIndex :type Integer) (bFromSweep :type Boolean) (SweepResult :type "HitResult Structure (by ref)"))
  (bind _as_bp_third_person_game_mode (`self.As BP Third Person Game Mode`))
  (bind _cube1 (`self.Cube1`))
  (bind (_relativelocation_x _relativelocation_y _relativelocation_z) (`KismetMathLibrary.BreakVector` (`SceneComponent.RelativeLocation` _cube1)))
  (if (== OtherActor (`/Game/GD/ThirdPerson/Blueprints/BP_ThirdPersonGameMode.As BP Third Person Character` _as_bp_third_person_game_mode))
    (`/Engine/EditorBlueprintResources/StandardMacros.DoOnce` false
      (:`Completed`
        (set `/Game/GD/ThirdPerson/Blueprints/BP_ThirdPersonGameMode.Respawn_Point` (`self.K2_GetActorLocation`) _as_bp_third_person_game_mode)
        (`KismetSystemLibrary.MoveComponentTo` _cube1 (`KismetMathLibrary.MakeVector` _relativelocation_x _relativelocation_y (+ _relativelocation_z 100.0)) (struct) true true 0.5)))))

(fn `UserConstructionScript`)