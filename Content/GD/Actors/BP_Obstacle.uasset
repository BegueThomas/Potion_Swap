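; Obstacle actor that knocks the player back on overlap, with a spike type (Piques) that also deals damage and a gust type (Bourrasque) that only pushes.
; Cube overlap checks for the player's capsule or lizard parts via the GameMode's PlayerRef; all three player forms currently react identically.
; The push launches along the Arrow when FixedDirection is set, otherwise backward from the player's facing, adding up or down force when a sphere trace hits a horizontal surface.
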(event `self.ReceiveBeginPlay`
  (bind _asbp_third_person_game_mode (cast `/Game/GD/ThirdPerson/Blueprints/BP_ThirdPersonGameMode` (`GameplayStatics.GetGameMode`)))
  (set `self.As BP Third Person Game Mode` _asbp_third_person_game_mode))

(event `self.Cube.OnComponentBeginOverlap`
  (params (OverlappedComponent :type "PrimitiveComponent Object Reference") (OtherActor :type "Actor Object Reference") (OtherComp :type "PrimitiveComponent Object Reference") (OtherBodyIndex :type Integer) (bFromSweep :type Boolean) (SweepResult :type "HitResult Structure (by ref)"))
  (bind _strenght_knockback (`self.Strenght_Knockback`))
  (bind _player_ref (`/Game/GD/ThirdPerson/Blueprints/BP_ThirdPersonGameMode.Player_Ref` (`self.As BP Third Person Game Mode`)))
  (if (or (== OtherComp (`Character.CapsuleComponent` _player_ref)) (== OtherComp (`/Game/GD/ThirdPerson/Blueprints/BP_ThirdPersonCharacter.Lizard_Bod` _player_ref)) (== OtherComp (`/Game/GD/ThirdPerson/Blueprints/BP_ThirdPersonCharacter.Lizard_Head` _player_ref)))
    (switch `/Game/GD/Input/Enum_Form` (`/Game/GD/ThirdPerson/Blueprints/BP_ThirdPersonCharacter.Enum_Form` _player_ref)
      (:`NewEnumerator0`
        (switch `/Game/GD/Actors/Enum_Obstacles` (`self.Obstacle_Type`)
          (:`NewEnumerator0`
            (`self.Event_push` _strenght_knockback :!label _label)
            (`/Game/GD/ThirdPerson/Blueprints/BP_ThirdPersonCharacter.Event_Reduce_Health` _player_ref (`self.Dégats`)))
          (:`NewEnumerator3`
            (`self.Event_push` _strenght_knockback :!label _label_2))))
      (:`NewEnumerator1`
        (switch `/Game/GD/Actors/Enum_Obstacles` (`self.Obstacle_Type`)
          (:`NewEnumerator0`
            (goto _label))
          (:`NewEnumerator3`
            (goto _label_2))))
      (:`NewEnumerator2`
        (switch `/Game/GD/Actors/Enum_Obstacles` (`self.Obstacle_Type`)
          (:`NewEnumerator0`
            (goto _label))
          (:`NewEnumerator3`
            (goto _label_2)))))))

(event `Event_push`
  (params (Push_Strenght :type "Float (double-precision)" :default -3000.0))
  (bind _player_ref (`/Game/GD/ThirdPerson/Blueprints/BP_ThirdPersonGameMode.Player_Ref` (`self.As BP Third Person Game Mode`)))
  (bind _returnvalue (`self.K2_GetActorLocation` (`/Game/GD/ThirdPerson/Blueprints/BP_ThirdPersonGameMode.Player_Ref` (`self.As BP Third Person Game Mode`))))
  (bind (_returnvalue_x _returnvalue_y _returnvalue_z) (`KismetMathLibrary.BreakVector` (* (`SceneComponent.GetForwardVector` (`self.Arrow`)) Push_Strenght)))
  (bind _capsulecomponent (`Character.CapsuleComponent` _player_ref))
  (bind _returnvalue_2 (`SceneComponent.GetUpVector` _capsulecomponent))
  (bind _returnvalue_3 (`SceneComponent.GetForwardVector` _capsulecomponent))
  (bind _returnvalue_4 (* _returnvalue_3 -2000.0))
  (if (`self.FixedDirection`)
    (`Character.LaunchCharacter` _player_ref (`KismetMathLibrary.MakeVector` _returnvalue_x _returnvalue_y (* _returnvalue_z 2.0)) true false)
    (else
      (bind (_outhit _returnvalue_5) (`KismetSystemLibrary.SphereTraceSingle` :`Start` _returnvalue :`End` _returnvalue :`Radius` 200.0 :`TraceChannel` "TraceTypeQuery4" :`bIgnoreSelf` false))
      (if _returnvalue_5
        (bind _z (.z (`.ImpactNormal` (`GameplayStatics.BreakHitResult` _outhit))))
        (`KismetSystemLibrary.PrintString` (`KismetStringLibrary.Conv_DoubleToString` _z))
        (if (== _z 1.0)
          (`Character.LaunchCharacter` _player_ref (+ (* _returnvalue_2 1000.0) _returnvalue_4) true false)
          (elif (== _z -1.0)
            (`Character.LaunchCharacter` _player_ref (+ (* _returnvalue_2 -1000.0) _returnvalue_4) true false)
            (else
              (`Character.LaunchCharacter` _player_ref (* _returnvalue_3 -3000.0) true false))))))))

(fn `UserConstructionScript`)