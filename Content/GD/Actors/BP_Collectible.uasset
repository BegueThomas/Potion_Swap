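; Collectible pickup actor that awards a coin to the player and destroys itself when the player overlaps its Overlap or Sphere component.
; Entering Zone_Magnet sets a flag that makes Tick stop InterpToMovement and ease the Sphere toward the player's location with MoveComponentTo.
; The GoldStatue flag swaps in a diamond mesh at construction and is passed to EventGainCoin.
; Spin and timer-driven bob logic is left unconnected.
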(event `self.ReceiveBeginPlay`
  (bind _asbp_third_person_game_mode (cast `/Game/GD/ThirdPerson/Blueprints/BP_ThirdPersonGameMode` (`GameplayStatics.GetGameMode`)))
  (set `self.As BP Third Person Game Mode` _asbp_third_person_game_mode))

(event `AnimCoin`
  (bind _sphere (`self.Sphere`))
  (bind (_returnvalue_x _returnvalue_y _returnvalue_z) (`KismetMathLibrary.BreakVector` (`SceneComponent.K2_GetComponentLocation` _sphere)))
  (bind (_direction _move) (`Timeline|Anim_Timeline` :!via `PlayFromStart`)
    (:`Update`
      (`SceneComponent.K2_SetWorldLocation` _sphere (`KismetMathLibrary.MakeVector` _returnvalue_x _returnvalue_y (+ _returnvalue_z _move)) false false))))

(event `self.Overlap.OnComponentBeginOverlap`
  (params (OverlappedComponent :type "PrimitiveComponent Object Reference") (OtherActor :type "Actor Object Reference") (OtherComp :type "PrimitiveComponent Object Reference") (OtherBodyIndex :type Integer) (bFromSweep :type Boolean) (SweepResult :type "HitResult Structure (by ref)"))
  (bind _player_ref (`/Game/GD/ThirdPerson/Blueprints/BP_ThirdPersonGameMode.Player_Ref` (`self.As BP Third Person Game Mode`)))
  (if (== OtherActor _player_ref)
    (`/Game/GD/ThirdPerson/Blueprints/BP_ThirdPersonCharacter.Event_GainCoin` _player_ref (`self.GoldStatue?`) :!label _label)
    (`self.K2_DestroyActor`)))

(event `self.Sphere.OnComponentBeginOverlap`
  (params (OverlappedComponent :type "PrimitiveComponent Object Reference") (OtherActor :type "Actor Object Reference") (OtherComp :type "PrimitiveComponent Object Reference") (OtherBodyIndex :type Integer) (bFromSweep :type Boolean) (SweepResult :type "HitResult Structure (by ref)"))
  (if (== OtherActor (`/Game/GD/ThirdPerson/Blueprints/BP_ThirdPersonGameMode.Player_Ref` (`self.As BP Third Person Game Mode`)))
    (goto _label)))

(event `self.Zone_Magnet.OnComponentBeginOverlap`
  (params (OverlappedComponent :type "PrimitiveComponent Object Reference") (OtherActor :type "Actor Object Reference") (OtherComp :type "PrimitiveComponent Object Reference") (OtherBodyIndex :type Integer) (bFromSweep :type Boolean) (SweepResult :type "HitResult Structure (by ref)"))
  (if (== OtherActor (`/Game/GD/ThirdPerson/Blueprints/BP_ThirdPersonGameMode.Player_Ref` (`self.As BP Third Person Game Mode`)))
    (set `self.Moving?` true)))

(event `self.ReceiveTick`
  (params (DeltaSeconds :type "Float (single-precision)"))
  (if (`self.Moving?`)
    (`ActorComponent.Deactivate` (`self.InterpToMovement`))
    (`KismetSystemLibrary.MoveComponentTo` (`self.Sphere`) (`self.K2_GetActorLocation` (`/Game/GD/ThirdPerson/Blueprints/BP_ThirdPersonGameMode.Player_Ref` (`self.As BP Third Person Game Mode`))) (struct) true false 2.0)))

(fn `UserConstructionScript`
  (if (`self.GoldStatue?`)
    (`StaticMeshComponent.SetStaticMesh` (`self.Sphere`) "/ControlRig/Controls/ControlRig_Diamond_solid.ControlRig_Diamond_solid")))