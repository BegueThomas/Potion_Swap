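; Camera zone actor that hands the view to its camera system component when the player capsule enters its box, locking the player camera until exit.
; Tick optionally turns the first camera toward the player and moves it along a spline, trailing the player's closest point.
; That point comes from a brute-force, unit-step search along the spline.
; With Distance set, overlaps are ignored and Activate runs a timed enter/exit instead.
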(event `self.ReceiveBeginPlay`
  (bind _asbp_third_person_game_mode (cast `/Game/GameDesign/ThirdPerson/Blueprints/BP_ThirdPersonGameMode` (`GameplayStatics.GetGameMode`)))
  (set `self.Ref_GameMode` _asbp_third_person_game_mode))

(event `self.ReceiveTick`
  (params (DeltaSeconds :type "Float (single-precision)"))
  (`self.RotateToPlayer`)
  (`self.FollowPlayer`))

(event `FollowPlayer`
  (bind _rootcomponent (`Actor.RootComponent` (`|GetArrayItem` (`/Game/Blueprint/ToolCamera/BPC_CameraSystem.AllCameraRef` (`self.BPC_CameraSystem`)))))
  (if (`self.Move?`)
    (bind _lenght (`self.GetClosestPosOnSpline` (`self.K2_GetActorLocation` (`/Game/GameDesign/ThirdPerson/Blueprints/BP_ThirdPersonGameMode.Player_Ref` (`self.Ref_GameMode`))) (`self.CameraSpeed`)))
    (`SceneComponent.K2_SetWorldLocation` _rootcomponent (`KismetMathLibrary.VLerp` (`SceneComponent.K2_GetComponentLocation` _rootcomponent) (`SplineComponent.GetLocationAtDistanceAlongSpline` (`self.Spline`) (`KismetMathLibrary.FMax` (- _lenght 1000.0)) "World") (* (`GameplayStatics.GetWorldDeltaSeconds`) (`self.CameraSpeed`))) false false)))

(event `self.Box.OnComponentBeginOverlap`
  (params (OverlappedComponent :type "PrimitiveComponent Object Reference") (OtherActor :type "Actor Object Reference") (OtherComp :type "PrimitiveComponent Object Reference") (OtherBodyIndex :type Integer) (bFromSweep :type Boolean) (SweepResult :type "HitResult Structure (by ref)"))
  (bind _player_ref (`/Game/GameDesign/ThirdPerson/Blueprints/BP_ThirdPersonGameMode.Player_Ref` (`self.Ref_GameMode`)))
  (if (== OtherComp (`Character.CapsuleComponent` _player_ref))
    (if (not (`self.Distance`))
      (`/Game/Blueprint/ToolCamera/BPC_CameraSystem.EnterTrigger` (`self.BPC_CameraSystem`) OtherActor (`self.Arrow`))
      (set `/Game/GameDesign/ThirdPerson/Blueprints/BP_ThirdPersonCharacter.CameraLock?` true _player_ref))))

(event `RotateToPlayer`
  (bind _rootcomponent (`Actor.RootComponent` (`|GetArrayItem` (`/Game/Blueprint/ToolCamera/BPC_CameraSystem.AllCameraRef` (`self.BPC_CameraSystem`)))))
  (if (`self.FocusOnPlayer`)
    (`SceneComponent.K2_SetWorldRotation` _rootcomponent (`KismetMathLibrary.RLerp` (`KismetMathLibrary.FindLookAtRotation` (`SceneComponent.K2_GetComponentLocation` _rootcomponent) (`self.K2_GetActorLocation` (`/Game/GameDesign/ThirdPerson/Blueprints/BP_ThirdPersonGameMode.Player_Ref` (`self.Ref_GameMode`)))) (`SceneComponent.K2_GetComponentRotation` _rootcomponent) (`GameplayStatics.GetWorldDeltaSeconds`)) false false)))

(event `self.Box.OnComponentEndOverlap`
  (params (OverlappedComponent :type "PrimitiveComponent Object Reference") (OtherActor :type "Actor Object Reference") (OtherComp :type "PrimitiveComponent Object Reference") (OtherBodyIndex :type Integer))
  (bind _player_ref (`/Game/GameDesign/ThirdPerson/Blueprints/BP_ThirdPersonGameMode.Player_Ref` (`self.Ref_GameMode`)))
  (if (== OtherComp (`Character.CapsuleComponent` _player_ref))
    (if (not (`self.Distance`))
      (`/Game/Blueprint/ToolCamera/BPC_CameraSystem.ExitTrigger` (`self.BPC_CameraSystem`) OtherActor)
      (set `/Game/GameDesign/ThirdPerson/Blueprints/BP_ThirdPersonCharacter.CameraLock?` false _player_ref))))

(event `/Game/ThirdPerson/BPI_Interact.Activate`
  (if (`self.Distance`)
    (`/Game/Blueprint/ToolCamera/BPC_CameraSystem.EnterTrigger` (`self.BPC_CameraSystem`) null null)
    (`Timeline|DELAY` :`NewTime` (`self.Time`)
      (:`Finished`
        (`/Game/Blueprint/ToolCamera/BPC_CameraSystem.ExitTrigger` (`self.BPC_CameraSystem`) (`GameplayStatics.GetPlayerPawn` 0))
        (`KismetSystemLibrary.PrintString` "Hello")))))

(fn `GetClosestPosOnSpline`
  (params (Location :type "Vector Structure") (Speed :type "Float (double-precision)" :default 20.0))
  (returns (Lenght :type "Float (double-precision)"))
  (locals (CheckLength :type "Float (double-precision)") (ClosestDistance :type "Float (double-precision)" :default 1000000000000000.0) (LenghtAtClosest :type "Float (double-precision)"))
  (bind _spline (`self.Spline`))
  (bind _checklength (`local.CheckLength`))
  (bind _checklength_2 (`local.CheckLength`))
  (bind _returnvalue (`KismetMathLibrary.Vector_Distance` (`SplineComponent.GetLocationAtDistanceAlongSpline` _spline _checklength "World") (`local.Location`)))
  (if (< _checklength (`SplineComponent.GetSplineLength` _spline)) :!label _label
    (if (> (`local.ClosestDistance`) _returnvalue)
      (bind _output_get (set `local.ClosestDistance` _returnvalue))
      (set `local.LenghtAtClosest` _checklength_2))
    (set `local.CheckLength` (+ _checklength_2 1.0))
    (`KismetSystemLibrary.PrintString` (`KismetStringLibrary.Conv_DoubleToString` _output_get) true false (struct :`R` 1.0 :`G` 0.699883 :`B` 0.040293 :`A` 1.0) 0.1)
    (goto _label)
    (else
      (return (`local.LenghtAtClosest`)))))

(fn `Held`
  (params (Origin :type "Vector Structure"))
  (returns (Origin_point :type "Vector Structure"))
  (return (0.0 0.0 0.0)))

(fn `UserConstructionScript`)