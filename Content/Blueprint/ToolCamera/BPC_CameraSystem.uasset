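; Actor component that switches the player's view to cine cameras on trigger events and can play a cinematic.
; On BeginPlay, if the game mode is BP_ThirdPersonGameMode, it spawns and attaches a CineCameraActor at each BPS_LocationCamera on its owner.
; EnterTrigger blends to the first camera and aligns control rotation to the supplied arrow; ExitTrigger blends back to the overlapping actor.
; PlayCinematic plays only the first sequence in its Cinematic array.
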(event `self.ReceiveBeginPlay`
  (bind _asbp_third_person_game_mode (cast `/Game/GameDesign/ThirdPerson/Blueprints/BP_ThirdPersonGameMode` (`GameplayStatics.GetGameMode`)))
  (set `self.Ref_GameMode` _asbp_third_person_game_mode)
  ; Initialization
  (bind _output_get (set `self.RefOwner` (`self.GetOwner`)))
  (bind _output_get_2 (set `self.Al_SocketCamera` (`Actor.K2_GetComponentsByClass` _output_get "/Game/Blueprint/ToolCamera/BPS_LocationCamera.BPS_LocationCamera_C")))
  ; Create Cine camera
  (for _array_element _output_get_2
    (bind _returnvalue (`|SpawnActorFromClass` "/Script/CinematicCamera.CineCameraActor" (`SceneComponent.K2_GetComponentToWorld` _array_element) "AlwaysSpawn" "MultiplyWithRoot" null null))
    (`KismetArrayLibrary.Array_Add` (`self.AllCameraRef`) _returnvalue)
    (`Actor.K2_AttachToComponent` _returnvalue _array_element "None" "KeepWorld" "KeepWorld" "KeepWorld" true)))

(event `EnterTrigger`
  (params (ActorOverlap :type "Actor Object Reference") (Arrow :type "ArrowComponent Object Reference"))
  (bind _returnvalue (`GameplayStatics.GetPlayerController` 0))
  ; Cinema
  (`PlayerController.SetViewTargetWithBlend` _returnvalue (`|GetArrayItem` (`self.AllCameraRef`)) (`self.Enter_TransitionTime`) (`self.Enter_Blend Func`) 0.0 false)
  (`Controller.SetControlRotation` _returnvalue (`SceneComponent.K2_GetComponentRotation` Arrow)))

(event `PlayCinematic`
  ; Cinematic
  (`MovieSceneSequencePlayer.Play` (`LevelSequenceActor.SequencePlayer` (`|GetArrayItem` (`self.Cinematic`)))))

(event `ExitTrigger`
  (params (ActorOverlap :type "Actor Object Reference"))
  ; Cinema
  (`PlayerController.SetViewTargetWithBlend` (`GameplayStatics.GetPlayerController` 0) ActorOverlap (`self.Exit_TransitionTime`) (`self.Exit_Blend Func`) 0.0 false))