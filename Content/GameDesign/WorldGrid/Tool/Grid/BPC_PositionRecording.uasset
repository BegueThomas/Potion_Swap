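; Actor component that records its owner's grid-snapped position into the BP_WorldGrid actor's map.
; On BeginPlay it reads grid size and refresh time from that actor, then starts a looping timer unless DontSave is set.
; SavePosition lowers the location one cell in Z, snaps it, then calls SaveInMap on the grid.
; SaveLevelTM calls the grid's Quit for game exit.
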(event `self.ReceiveBeginPlay`
  (bind _returnvalue (`GameplayStatics.GetActorOfClass` "/Game/GameDesign/WorldGrid/Tool/Grid/BP_WorldGrid.BP_WorldGrid_C"))
  (bind _output_get (set `self.WorldGridActor` _returnvalue))
  (`/Engine/EditorBlueprintResources/StandardMacros.IsValid` _output_get
    (:`Is Valid`
      (set `self.GridSize` (`/Game/GameDesign/WorldGrid/Tool/Grid/BP_WorldGrid.GridSize_WG` _output_get))
      (set `self.RefreshTime` (`/Game/GameDesign/WorldGrid/Tool/Grid/BP_WorldGrid.RefreshTime` _output_get))
      (if (not (`/Game/GameDesign/WorldGrid/Tool/Grid/BP_WorldGrid.DontSave` _output_get))
        (`KismetSystemLibrary.K2_SetTimerDelegate` (`|CreateDelegate` :!event `SavePosition`) (`self.RefreshTime`) true)))))

(event `SaveLevelTM`
  ; NeedExit Game Event
  (bind _returnvalue (`GameplayStatics.GetActorOfClass` "/Game/GameDesign/WorldGrid/Tool/Grid/BP_WorldGrid.BP_WorldGrid_C"))
  (bind _output_get (set `self.WorldGridActor` _returnvalue))
  (`/Game/GameDesign/WorldGrid/Tool/Grid/BP_WorldGrid.Quit` _output_get))

(fn `SavePosition`
  (bind _worldgridactor (`self.WorldGridActor`))
  (bind _output_get (set `self.CurrentPosition` (`KismetMathLibrary.Vector_SnappedToGrid` (- (`Actor.K2_GetActorLocation` (`self.GetOwner`)) (`KismetMathLibrary.MakeVector` 0.0 0.0 (`self.GridSize`))) (`self.GridSize`))))
  (set `/Game/GameDesign/WorldGrid/Tool/Grid/BP_WorldGrid.Location` _output_get _worldgridactor)
  (`/Game/GameDesign/WorldGrid/Tool/Grid/BP_WorldGrid.SaveInMap` _worldgridactor)
  (return))