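; BP_NotifySteps is an animation notify that plays a footstep sound matching the surface under the player.
; It line traces 100 units down from player pawn 0, rather than the animated mesh, and switches on the hit physical material's surface type.
; Grass has its own sound, Dirt and Snow share a wood sound, Mud and Water share a water sound, and other surfaces use a default cue, all played in 2D.
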(fn `Received_Notify`
  (params (MeshComp :type "SkeletalMeshComponent Object Reference") (Animation :type "AnimSequenceBase Object Reference") (EventReference :type "AnimNotifyEventReference Structure (by ref)"))
  (returns (ReturnValue :type Boolean))
  (bind _returnvalue (`Actor.K2_GetActorLocation` (`GameplayStatics.GetPlayerPawn` 0)))
  (bind _outhit (`KismetSystemLibrary.LineTraceSingle` _returnvalue (`KismetMathLibrary.MakeVector` (.x _returnvalue) (.y _returnvalue) (+ (.z _returnvalue) -100.0)) "TraceTypeQuery1"))
  (switch `EPhysicalSurface` (`PhysicalMaterial.SurfaceType` (`.PhysMat` (`GameplayStatics.BreakHitResult` _outhit)))
    (:`SurfaceType_Default`
      (`GameplayStatics.PlaySound2D` "/Game/SoundDesign/PlaceHolder/SFX/Marche_Bleu_SFX/Marche_Bleu_Cue.Marche_Bleu_Cue" 1.0 1.0 0.0 null null))
    (:`SurfaceType1`
      (`GameplayStatics.PlaySound2D` "/Game/SoundDesign/PlaceHolder/SFX/Marche_Bleu_SFX/vfx_grass.vfx_grass" 2.0 1.0 0.0 null null)
      (return false))
    (:`SurfaceType2`
      (`GameplayStatics.PlaySound2D` "/Game/SoundDesign/PlaceHolder/SFX/Marche_Bleu_SFX/vfx_wood.vfx_wood" 1.0 1.0 3.8 null null :!label _label)
      (return false))
    (:`SurfaceType3`
      (`GameplayStatics.PlaySound2D` "/Game/SoundDesign/PlaceHolder/SFX/Marche_Bleu_SFX/vfx_water.vfx_water" 1.0 1.0 14.2 null null :!label _label_2))
    (:`SurfaceType4`
      (goto _label))
    (:`SurfaceType5`
      (goto _label_2))))