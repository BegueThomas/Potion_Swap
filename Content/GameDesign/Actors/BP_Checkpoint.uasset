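; Checkpoint actor that updates the player's respawn point the first time the player touches it.
; BeginPlay caches BP_ThirdPersonGameMode, and the Box overlap compares the other actor to its PlayerRef.
; A DoOnce then writes the game mode's RespawnPoint from the Box location and Arrow rotation and plays a checkpoint sound.
; An eased MoveComponentTo that would raise a component is left unconnected.
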(event `self.ReceiveBeginPlay`
  (bind _asbp_third_person_game_mode (cast `/Game/GameDesign/ThirdPerson/Blueprints/BP_ThirdPersonGameMode` (`GameplayStatics.GetGameMode`)))
  (set `self.As BP Third Person Game Mode` _asbp_third_person_game_mode))

(event `self.Box.OnComponentBeginOverlap`
  (params (OverlappedComponent :type "PrimitiveComponent Object Reference") (OtherActor :type "Actor Object Reference") (OtherComp :type "PrimitiveComponent Object Reference") (OtherBodyIndex :type Integer) (bFromSweep :type Boolean) (SweepResult :type "HitResult Structure (by ref)"))
  (bind _as_bp_third_person_game_mode (`self.As BP Third Person Game Mode`))
  (if (== OtherActor (`/Game/GameDesign/ThirdPerson/Blueprints/BP_ThirdPersonGameMode.Player_Ref` _as_bp_third_person_game_mode))
    (`/Engine/EditorBlueprintResources/StandardMacros.DoOnce` false
      (:`Completed`
        (set `/Game/GameDesign/ThirdPerson/Blueprints/BP_ThirdPersonGameMode.Respawn_Point` (`KismetMathLibrary.MakeTransform` (`SceneComponent.K2_GetComponentLocation` (`self.Box`)) (`SceneComponent.K2_GetComponentRotation` (`self.Arrow`))) _as_bp_third_person_game_mode)
        (`GameplayStatics.PlaySound2D` "/Game/SoundDesign/PlaceHolder/SFX/SFX_Checkpoint.SFX_Checkpoint" 1.0 1.0 0.0 null null)))))

(fn `UserConstructionScript`)