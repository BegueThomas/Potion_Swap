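; BP_Platform is a moving platform whose mesh oscillates around its start position by a configurable Movement vector.
; BeginPlay computes both endpoints and starts a looping timer that replays two chained, eased MoveComponentTo legs.
; An unconnected player-contact reaction would halt the motion, dip the platform and restart it.
; The Suspension function applies trace-based spring forces to a physics Box at one or several points, but its call is also unconnected.
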(event `self.ReceiveBeginPlay`
  (bind _returnvalue (* (`self.Movement`) 1.0))
  (bind _relativelocation (`SceneComponent.RelativeLocation` (`self.SM_Plateform_A`)))
  (bind _asbp_third_person_game_mode (cast `/Game/GameDesign/ThirdPerson/Blueprints/BP_ThirdPersonGameMode` (`GameplayStatics.GetGameMode`)))
  (set `self.As BP Third Person Game Mode` _asbp_third_person_game_mode)
  (set `self.Up_Vector` (+ _relativelocation _returnvalue))
  (set `self.Down_Vector` (+ _relativelocation (* _returnvalue -1.0)))
  (`self.Movement_Event`)
  (bind _returnvalue_2 (`KismetSystemLibrary.K2_SetTimerDelegate` (delegate `Movement_Event`) 4.0 true))
  (set `self.Timer_Handle` _returnvalue_2))

(event `Movement_Event`
  (`KismetSystemLibrary.MoveComponentTo` (`self.SM_Plateform_A`) (`self.Up_Vector`) (struct) true true 2.0)
  (`KismetSystemLibrary.MoveComponentTo` (`self.SM_Plateform_A`) (`self.Down_Vector`) (struct) true true 2.0))

(event `self.Box.OnComponentBeginOverlap`
  (params (OverlappedComponent :type "PrimitiveComponent Object Reference") (OtherActor :type "Actor Object Reference") (OtherComp :type "PrimitiveComponent Object Reference") (OtherBodyIndex :type Integer) (bFromSweep :type Boolean) (SweepResult :type "HitResult Structure (by ref)")))

(event `self.ReceiveTick`
  (params (DeltaSeconds :type "Float (single-precision)")))

(fn `Suspension`
  (params (Target :type "SceneComponent Object Reference"))
  (bind _returnvalue (`SceneComponent.K2_GetComponentLocation` Target))
  (bind _distance_ground (`self.Distance_Ground`))
  (bind _returnvalue_2 (+ _returnvalue (`SceneComponent.RelativeLocation` Target)))
  (`PrimitiveComponent.SetSimulatePhysics` (`self.Box`) true)
  (if (`self.Multi?`)
    (for _array_element (`self.ListPoint`)
      (bind _returnvalue_3 (+ _array_element _returnvalue))
      (bind _outhit (`KismetSystemLibrary.LineTraceSingle` :`Start` _returnvalue_3 :`End` (- _returnvalue_3 (`KismetMathLibrary.MakeVector` 0.0 0.0 _distance_ground)) :`TraceChannel` "TraceTypeQuery1" :`DrawDebugType` "ForOneFrame"))
      (bind (_bblockinghit _binitialoverlap _time _distance _location _impactpoint _normal _impactnormal _physmat _hitactor _hitcomponent _hitbonename _bonename _hititem _elementindex _faceindex _tracestart _traceend) (`GameplayStatics.BreakHitResult` _outhit))
      (if _bblockinghit
        (`PrimitiveComponent.AddForceAtLocation` (`self.Box`) (* (- 1.0 (`KismetMathLibrary.NormalizeToRange` _distance 0.0 (`self.Range Max`))) (`KismetMathLibrary.GetDirectionUnitVector` _traceend _tracestart) (`self.ForceMulti`)) _returnvalue_3 "None")))
    (else
      (bind _outhit_2 (`KismetSystemLibrary.LineTraceSingle` :`Start` _returnvalue_2 :`End` (- _returnvalue_2 (`KismetMathLibrary.MakeVector` 0.0 0.0 _distance_ground)) :`TraceChannel` "TraceTypeQuery1" :`DrawDebugType` "ForOneFrame"))
      (bind (_bblockinghit_2 _binitialoverlap_2 _time_2 _distance_2 _location_2 _impactpoint_2 _normal_2 _impactnormal_2 _physmat_2 _hitactor_2 _hitcomponent_2 _hitbonename_2 _bonename_2 _hititem_2 _elementindex_2 _faceindex_2 _tracestart_2 _traceend_2) (`GameplayStatics.BreakHitResult` _outhit_2))
      (if _bblockinghit_2
        (`PrimitiveComponent.AddForceAtLocation` (`self.Box`) (* (- 1.0 (`KismetMathLibrary.NormalizeToRange` _distance_2 0.0 (`self.Range Max`))) (`KismetMathLibrary.GetDirectionUnitVector` _traceend_2 _tracestart_2) (`self.ForceMulti`)) _returnvalue_2 "None")))))

(fn `UserConstructionScript`)