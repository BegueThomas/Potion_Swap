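; BP_Collectible is a pickup whose category (coin, gold statue, red or green fruit, victory) sets its mesh and, mostly, material in the Construction Script.
; Entering Zone_Magnet sets a flag that makes Tick stop InterpToMovement and ease the Sphere toward the player's location.
; Player overlap with Overlap or Sphere calls EventGainCoin with the category, then destroys the actor.
; The timeline bob and spin logic are left unhooked.
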(event `self.ReceiveBeginPlay`
  (bind _asbp_third_person_game_mode (cast `/Game/GameDesign/ThirdPerson/Blueprints/BP_ThirdPersonGameMode` (`GameplayStatics.GetGameMode`)))
  (set `self.As BP Third Person Game Mode` _asbp_third_person_game_mode))

(event `AnimCoin`
  (bind _sphere (`self.Sphere`))
  (bind (_returnvalue_x _returnvalue_y _returnvalue_z) (`KismetMathLibrary.BreakVector` (`SceneComponent.K2_GetComponentLocation` _sphere)))
  (bind (_direction _move) (`Timeline|Anim_Timeline` :!via `PlayFromStart`)
    (:`Update`
      (`SceneComponent.K2_SetWorldLocation` _sphere (`KismetMathLibrary.MakeVector` _returnvalue_x _returnvalue_y (+ _returnvalue_z _move)) false false))))

(event `self.Overlap.OnComponentBeginOverlap`
  (params (OverlappedComponent :type "PrimitiveComponent Object Reference") (OtherActor :type "Actor Object Reference") (OtherComp :type "PrimitiveComponent Object Reference") (OtherBodyIndex :type Integer) (bFromSweep :type Boolean) (SweepResult :type "HitResult Structure (by ref)"))
  (if (== OtherActor (`/Game/GameDesign/ThirdPerson/Blueprints/BP_ThirdPersonGameMode.Player_Ref` (`self.As BP Third Person Game Mode`)))
    (`/Game/GameDesign/ThirdPerson/Blueprints/BP_ThirdPersonCharacter.Event_GainCoin` (`/Game/GameDesign/ThirdPerson/Blueprints/BP_ThirdPersonGameMode.Player_Ref` (`self.As BP Third Person Game Mode`)) (`self.Category`) :!label _label)
    (`self.K2_DestroyActor`)))

(event `self.Sphere.OnComponentBeginOverlap`
  (params (OverlappedComponent :type "PrimitiveComponent Object Reference") (OtherActor :type "Actor Object Reference") (OtherComp :type "PrimitiveComponent Object Reference") (OtherBodyIndex :type Integer) (bFromSweep :type Boolean) (SweepResult :type "HitResult Structure (by ref)"))
  (if (== OtherActor (`/Game/GameDesign/ThirdPerson/Blueprints/BP_ThirdPersonGameMode.Player_Ref` (`self.As BP Third Person Game Mode`)))
    (goto _label)))

(event `self.Zone_Magnet.OnComponentBeginOverlap`
  (params (OverlappedComponent :type "PrimitiveComponent Object Reference") (OtherActor :type "Actor Object Reference") (OtherComp :type "PrimitiveComponent Object Reference") (OtherBodyIndex :type Integer) (bFromSweep :type Boolean) (SweepResult :type "HitResult Structure (by ref)"))
  (if (== OtherActor (`/Game/GameDesign/ThirdPerson/Blueprints/BP_ThirdPersonGameMode.Player_Ref` (`self.As BP Third Person Game Mode`)))
    (set `self.Moving?` true)))

(event `self.ReceiveTick`
  (params (DeltaSeconds :type "Float (single-precision)"))
  (if (`self.Moving?`)
    (`ActorComponent.Deactivate` (`self.InterpToMovement`))
    (`KismetSystemLibrary.MoveComponentTo` (`self.Sphere`) (`self.K2_GetActorLocation` (`/Game/GameDesign/ThirdPerson/Blueprints/BP_ThirdPersonGameMode.Player_Ref` (`self.As BP Third Person Game Mode`))) (struct) true false 2.0)))

(fn `UserConstructionScript`
  (bind _sphere (`self.Sphere`))
  (bind _sphere_2 (`self.Sphere`))
  (switch `/Game/GameDesign/Actors/Enum_Collectibles` (`self.Category`)
    (:`NewEnumerator0`
      (`StaticMeshComponent.SetStaticMesh` _sphere_2 "/Game/GameDesign/PlaceHolders/PH_Mesh_Coin.PH_Mesh_Coin")
      (`PrimitiveComponent.SetMaterial` _sphere_2 0 "/Game/GameDesign/PlaceHolders/Mat_PH.Mat_PH"))
    (:`NewEnumerator1`
      (`StaticMeshComponent.SetStaticMesh` (`self.Sphere`) "/ControlRig/Controls/ControlRig_Diamond_solid.ControlRig_Diamond_solid"))
    (:`NewEnumerator2`
      (`StaticMeshComponent.SetStaticMesh` _sphere "/ControlRig/Controls/ControlRig_Sphere_solid.ControlRig_Sphere_solid")
      (`PrimitiveComponent.SetMaterial` _sphere 0 "/AnimationSharing/AnimSharingRed.AnimSharingRed"))
    (:`NewEnumerator4`
      (`StaticMeshComponent.SetStaticMesh` _sphere "/ControlRig/Controls/ControlRig_Sphere_solid.ControlRig_Sphere_solid")
      (`PrimitiveComponent.SetMaterial` _sphere 0 "/AnimationSharing/AnimSharingGreen.AnimSharingGreen"))
    (:`NewEnumerator3`
      (`StaticMeshComponent.SetStaticMesh` _sphere "/Engine/VREditor/BasicMeshes/SM_Pyramid_01.SM_Pyramid_01")
      (`PrimitiveComponent.SetMaterial` _sphere 0 "/Engine/VREditor/UI/ArrowMaterial.ArrowMaterial"))))