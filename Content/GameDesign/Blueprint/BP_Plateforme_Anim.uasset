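; Animated platform that moves its TriggerBox along a spline using the Anim timeline and a curve, with play rate set by Duration.
; Activate toggles play and stop, gated by an Ongoing flag when not looping.
; Horizontal moves sweep and push blocking actors by the remaining distance in XY; other moves teleport-free without sweep.
; Tick runs Suspension, enabling physics and applying distance-scaled hover forces from single or multiple downward line traces.
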(event `self.ReceiveTick`
  (params (DeltaSeconds :type "Float (single-precision)"))
  (if (`self.Anim?`)
    (`self.Suspension` (`self.Pivot_Point`))))

(event `self.ReceiveBeginPlay`
  (bind _anim (`self.Anim`))
  ; Set animation play rate
  (`TimelineComponent.SetPlayRate` _anim (/ 1.0 (`self.Duration`)))
  (`TimelineComponent.SetLooping` _anim (`self.Loop?`)))

(event `/Game/ThirdPerson/BPI_Interact.Activate`
  (bind _spline (`self.Spline`))
  (bind _trigger_box (`self.Trigger_Box`))
  (bind _ongoing_ (`self.Ongoing?`))
  (if (`self.Loop?`)
    (`/Engine/EditorBlueprintResources/StandardMacros.FlipFlop`
      (:`A`
        (bind (_direction _percent_anim) (`Timeline|Anim` :!label _label)
          (:`Update`
            (bind _returnvalue (`SplineComponent.GetLocationAtDistanceAlongSpline` _spline (* (`CurveFloat.GetFloatValue` (`self.CurveAnim`) _percent_anim) (`SplineComponent.GetSplineLength` _spline)) "World"))
            (bind (_returnvalue_x _returnvalue_y _returnvalue_z) (`KismetMathLibrary.BreakVector` (`KismetMathLibrary.GetDirectionUnitVector` _returnvalue (`SceneComponent.K2_GetComponentLocation` _trigger_box))))
            (if (== _returnvalue_z 0.0)
              (bind _sweephitresult (`SceneComponent.K2_SetWorldLocation` (`self.Trigger_Box`) _returnvalue true false))
              (bind (_bblockinghit _binitialoverlap _time _distance _location _impactpoint _normal _impactnormal _physmat _hitactor _hitcomponent _hitbonename _bonename _hititem _elementindex _faceindex _tracestart _traceend) (`GameplayStatics.BreakHitResult` _sweephitresult))
              (if _bblockinghit
                (bind (_returnvalue_x_2 _returnvalue_y_2) (`KismetMathLibrary.BreakVector` (* (`KismetMathLibrary.GetDirectionUnitVector` _tracestart _traceend) (- (`KismetMathLibrary.Vector_Distance` _tracestart _traceend) _distance))))
                (`self.K2_AddActorWorldOffset` _hitactor (`KismetMathLibrary.MakeVector` _returnvalue_x_2 _returnvalue_y_2) true false))
              (else
                (`SceneComponent.K2_SetWorldLocation` _trigger_box _returnvalue false false))))
          (:`Finished`
            (set `self.Ongoing?` false))))
      (:`B`
        (goto _label :!via `Stop`)))
    (elif (`self.Position?`)
      (if (not _ongoing_)
        (set `self.Position?` false)
        (set `self.Ongoing?` true)
        (goto _label))
      (elif (not _ongoing_)
        (set `self.Position?` true)
        (set `self.Ongoing?` true)
        (goto _label :!via `Stop`)))))

(fn `Held`
  (params (Origin :type "Vector Structure"))
  (returns (Origin_point :type "Vector Structure"))
  (return (0.0 0.0 0.0)))

(fn `Suspension`
  (params (Pivot :type "SceneComponent Object Reference"))
  (bind _returnvalue (`SceneComponent.K2_GetComponentLocation` Pivot))
  (bind _distance_ground (`self.Distance_Ground`))
  (bind _returnvalue_2 (+ _returnvalue (`SceneComponent.RelativeLocation` Pivot)))
  (`PrimitiveComponent.SetSimulatePhysics` (`self.Trigger_Box`) true)
  (if (`self.Multi?`)
    (for _array_element (`self.ListPoint`)
      (bind _returnvalue_3 (+ _array_element _returnvalue))
      (bind _outhit (`KismetSystemLibrary.LineTraceSingle` _returnvalue_3 (- _returnvalue_2 (`KismetMathLibrary.MakeVector` 0.0 0.0 _distance_ground)) "TraceTypeQuery1"))
      (bind (_bblockinghit _binitialoverlap _time _distance _location _impactpoint _normal _impactnormal _physmat _hitactor _hitcomponent _hitbonename _bonename _hititem _elementindex _faceindex _tracestart _traceend) (`GameplayStatics.BreakHitResult` _outhit))
      (if _bblockinghit
        (`PrimitiveComponent.AddForceAtLocation` (`self.Trigger_Box`) (* (- 1.0 (`KismetMathLibrary.NormalizeToRange` _distance 0.0 (`self.Range Max`))) (`KismetMathLibrary.GetDirectionUnitVector` _traceend _tracestart) (`self.ForceMulti`)) _returnvalue_3 "None")))
    (else
      (bind _outhit_2 (`KismetSystemLibrary.LineTraceSingle` _returnvalue_2 (- _returnvalue_2 (`KismetMathLibrary.MakeVector` 0.0 0.0 _distance_ground)) "TraceTypeQuery1"))
      (bind (_bblockinghit_2 _binitialoverlap_2 _time_2 _distance_2 _location_2 _impactpoint_2 _normal_2 _impactnormal_2 _physmat_2 _hitactor_2 _hitcomponent_2 _hitbonename_2 _bonename_2 _hititem_2 _elementindex_2 _faceindex_2 _tracestart_2 _traceend_2) (`GameplayStatics.BreakHitResult` _outhit_2))
      (if _bblockinghit_2
        (`PrimitiveComponent.AddForceAtLocation` (`self.Trigger_Box`) (* (- 1.0 (`KismetMathLibrary.NormalizeToRange` _distance_2 0.0 (`self.Range Max`))) (`KismetMathLibrary.GetDirectionUnitVector` _traceend_2 _tracestart_2) (`self.ForceMulti`)) _returnvalue_2 "None")))))

(fn `UserConstructionScript`)