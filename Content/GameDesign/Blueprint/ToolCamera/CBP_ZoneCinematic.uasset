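; Trigger-zone Blueprint that plays a cinematic when the first player's pawn enters its box.
; On overlap, it calls PlayCinematic on its camera system component and switches the player controller to UI-only input.
; A delay based on the play length of the component's first Cinematic entry then restores game-only input.
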(event `self.Box.OnComponentBeginOverlap`
  (params (OverlappedComponent :type "PrimitiveComponent Object Reference") (OtherActor :type "Actor Object Reference") (OtherComp :type "PrimitiveComponent Object Reference") (OtherBodyIndex :type Integer) (bFromSweep :type Boolean) (SweepResult :type "HitResult Structure (by ref)"))
  (bind _returnvalue (`GameplayStatics.GetPlayerController` 0))
  (bind _bpc_camerasystem (`self.BPC_CameraSystem`))
  (if (== OtherActor (`GameplayStatics.GetPlayerPawn` 0))
    (if (`self.Once?`)
      (`/Engine/EditorBlueprintResources/StandardMacros.DoOnce` false
        (:`Completed`
          _)))
    (`/Game/GameDesign/Blueprint/ToolCamera/BPC_CameraSystem.PlayCinematic` _bpc_camerasystem)
    (`WidgetBlueprintLibrary.SetInputMode_UIOnlyEx` _returnvalue null)
    (bind _returnvalue_2 (message `AnimationDataModel.GetPlayLength` (`|GetArrayItem` (`/Game/GameDesign/Blueprint/ToolCamera/BPC_CameraSystem.Cinematic` _bpc_camerasystem))))
    (`KismetSystemLibrary.Delay` _returnvalue_2)
    (`WidgetBlueprintLibrary.SetInputMode_GameOnly` _returnvalue)))

(fn `UserConstructionScript`)