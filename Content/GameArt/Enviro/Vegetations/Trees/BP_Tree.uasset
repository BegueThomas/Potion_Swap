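; BP_Tree is a vegetation actor that builds a tree from a configurable trunk mesh and leaves mesh.
; Its construction script assigns each mesh to its own instanced static mesh component, clears old instances and adds one instance at the local origin with unit scale.
; The event graph has only disabled placeholder events, so the Blueprint runs no gameplay logic.
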(fn `UserConstructionScript`
  (bind _returnvalue (`KismetMathLibrary.MakeTransform` (0.0 0.0 0.0)))
  (bind _ism_trunk (`self.ISM_Trunk`))
  (bind _ism_leaves (`self.ISM_Leaves`))
  (`StaticMeshComponent.SetStaticMesh` _ism_trunk (`self.Trunk_Mesh`))
  (`InstancedStaticMeshComponent.ClearInstances` _ism_trunk)
  (`InstancedStaticMeshComponent.AddInstance` _ism_trunk _returnvalue false)
  (`StaticMeshComponent.SetStaticMesh` _ism_leaves (`self.Leaves_Mesh`))
  (`InstancedStaticMeshComponent.ClearInstances` _ism_leaves)
  (`InstancedStaticMeshComponent.AddInstance` _ism_leaves _returnvalue false))