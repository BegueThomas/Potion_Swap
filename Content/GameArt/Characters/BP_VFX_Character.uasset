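; BP_VFX_Character is a character effects Blueprint that plays the Niagara effect for switching between bird, quadruped and lizard transformations.
; The Switch_VFX event passes its selection to SwitchTransformation, which swaps the matching system onto a single Niagara component, resetting overridden parameters.
; It then activates that component without a forced reset and returns it.
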(event `Switch_VFX`
  (params (Selection :type "/Game/GameArt/Characters/E_VFX_Transformation Enum" :default "NewEnumerator0"))
  (`self.Switch_Transformation` Selection))

(fn `Switch_Transformation`
  (params (Selection :type "/Game/GameArt/Characters/E_VFX_Transformation Enum" :default "NewEnumerator0"))
  (returns (Niagara :type "NiagaraComponent Object Reference"))
  (switch `/Game/GameArt/Characters/E_VFX_Transformation` Selection
    (:`NewEnumerator0`
      (`NiagaraComponent.SetAsset` (`self.Niagara`) "/Game/GameArt/Characters/Bird/VFX/VFX_Switch/NS_Switch_Bird.NS_Switch_Bird" true))
    (:`NewEnumerator1`
      (`NiagaraComponent.SetAsset` (`self.Niagara`) "/Game/GameArt/Characters/Quadruped/VFX/VFX_Switch/NS_Switch_Quadruped.NS_Switch_Quadruped" true))
    (:`NewEnumerator2`
      (`NiagaraComponent.SetAsset` (`self.Niagara`) "/Game/GameArt/Characters/Lezard/VFX/VFX_Switch/NS_Switch_Lezard.NS_Switch_Lezard" true)))
  (`ActorComponent.Activate` (`self.Niagara`) false)
  (return (`self.Niagara`)))

(fn `UserConstructionScript`)