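; BP_ModularWalls is a procedural modular wall Blueprint that configures three wall pieces from a selected wall set.
; Its construction script switches on WallSet, with each set defining a different combination of widths for Wall1, Wall2 and Wall3.
; Each wall's variation index picks an entry from the array for that size, stored with a matching size value while keeping the variation.
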(fn `UserConstructionScript`
  (bind (_wall1_mesh _wall1_wallmesh _wall1_variation) (break `/Game/GameArt/TechArt/Procedural/Walls/Structures/S_WallList` (`self.Wall1`)))
  (bind (_wall2_mesh _wall2_wallmesh _wall2_variation) (break `/Game/GameArt/TechArt/Procedural/Walls/Structures/S_WallList` (`self.Wall2`)))
  (bind (_wall3_mesh _wall3_wallmesh _wall3_variation) (break `/Game/GameArt/TechArt/Procedural/Walls/Structures/S_WallList` (`self.Wall3`)))
  (bind (_wall1_mesh_2 _wall1_wallmesh_2 _wall1_variation_2) (break `/Game/GameArt/TechArt/Procedural/Walls/Structures/S_WallList` (`self.Wall1`)))
  (bind (_wall2_mesh_2 _wall2_wallmesh_2 _wall2_variation_2) (break `/Game/GameArt/TechArt/Procedural/Walls/Structures/S_WallList` (`self.Wall2`)))
  (bind (_wall3_mesh_2 _wall3_wallmesh_2 _wall3_variation_2) (break `/Game/GameArt/TechArt/Procedural/Walls/Structures/S_WallList` (`self.Wall3`)))
  (bind (_wall1_mesh_3 _wall1_wallmesh_3 _wall1_variation_3) (break `/Game/GameArt/TechArt/Procedural/Walls/Structures/S_WallList` (`self.Wall1`)))
  (bind (_wall2_mesh_3 _wall2_wallmesh_3 _wall2_variation_3) (break `/Game/GameArt/TechArt/Procedural/Walls/Structures/S_WallList` (`self.Wall2`)))
  (bind (_wall3_mesh_3 _wall3_wallmesh_3 _wall3_variation_3) (break `/Game/GameArt/TechArt/Procedural/Walls/Structures/S_WallList` (`self.Wall3`)))
  (switch `/Game/GameArt/TechArt/Procedural/Walls/Enums/E_WallSet` (`self.WallSet`)
    (:`NewEnumerator0`
      (set `self.Wall1` (make `/Game/GameArt/TechArt/Procedural/Walls/Structures/S_WallList` (`|GetArrayItem` (`self.Walls60`) _wall1_variation) 0.6 _wall1_variation))
      (set `self.Wall2` (make `/Game/GameArt/TechArt/Procedural/Walls/Structures/S_WallList` (`|GetArrayItem` (`self.Walls120`) _wall2_variation) 1.2 _wall2_variation))
      (set `self.Wall3` (make `/Game/GameArt/TechArt/Procedural/Walls/Structures/S_WallList` (`|GetArrayItem` (`self.Walls120`) _wall3_variation) 1.2 _wall3_variation)))
    (:`NewEnumerator1`
      (set `self.Wall1` (make `/Game/GameArt/TechArt/Procedural/Walls/Structures/S_WallList` (`|GetArrayItem` (`self.Walls80`) _wall1_variation_2) 0.8 _wall1_variation_2))
      (set `self.Wall2` (make `/Game/GameArt/TechArt/Procedural/Walls/Structures/S_WallList` (`|GetArrayItem` (`self.Walls100`) _wall2_variation_2) 1.0 _wall2_variation_2))
      (set `self.Wall3` (make `/Game/GameArt/TechArt/Procedural/Walls/Structures/S_WallList` (`|GetArrayItem` (`self.Walls120`) _wall3_variation_2) 1.2 _wall3_variation_2)))
    (:`NewEnumerator2`
      (set `self.Wall1` (make `/Game/GameArt/TechArt/Procedural/Walls/Structures/S_WallList` (`|GetArrayItem` (`self.Walls60`) _wall1_variation_3) 0.6 _wall1_variation_3))
      (set `self.Wall2` (make `/Game/GameArt/TechArt/Procedural/Walls/Structures/S_WallList` (`|GetArrayItem` (`self.Walls100`) _wall2_variation_3) 1.0 _wall2_variation_3))
      (set `self.Wall3` (make `/Game/GameArt/TechArt/Procedural/Walls/Structures/S_WallList` (`|GetArrayItem` (`self.Walls140`) _wall3_variation_3) 1.4 _wall3_variation_3)))))