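; BP_CableVines is a procedural vine actor that strings a cable component between two surfaces.
; The construction script traces backward from the actor and forward from the End component, ignoring other vines, and snaps each end to its hit.
; Cable length follows the span with random slack and drives a dynamic material's tiling.
; Vines lacking either attachment are hidden in game and flagged as unable to spawn.
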(fn `UserConstructionScript`
  (bind _returnvalue (`self.K2_GetActorLocation`))
  (bind _cable (`self.Cable`))
  (bind _end (`self.End`))
  (bind _returnvalue_2 (`SceneComponent.K2_GetComponentLocation` _end))
  (bind _returnvalue_3 (`KismetMathLibrary.Vector_Distance` (`SceneComponent.K2_GetComponentLocation` (`self.Cable`)) (`SceneComponent.K2_GetComponentLocation` (`self.End`))))
  (bind _returnvalue_4 (`PrimitiveComponent.CreateDynamicMaterialInstance` _cable 0 (`PrimitiveComponent.GetMaterial` _cable 0) "None"))
  (bind _output_get (set `self.DMI_Vines` _returnvalue_4))
  (`PrimitiveComponent.SetMaterial` _cable 0 _output_get)
  (bind _outactors (`GameplayStatics.GetAllActorsOfClass` "BP_CableVines_C"))
  (set `self.Out Actors` _outactors)
  (set `CableComponent.CableLength` (`self.Cable Length`) (`self.Cable`))
  (set `self.CableLengthMult` (`KismetMathLibrary.RandomFloatInRange` 0.4 1.0))
  (`|ExecutionSequence`
    (:`then_0`
      (bind _outhit (`KismetSystemLibrary.LineTraceSingle` _returnvalue (+ _returnvalue (* (`self.GetActorForwardVector`) (`self.TraceDistance`) -1.0)) "TraceTypeQuery1" false (`self.Out Actors`) "None" true (struct :`R` 1.0 :`A` 1.0) (struct :`G` 1.0 :`A` 1.0) 1.0))
      (bind (_bblockinghit _binitialoverlap _time _distance _location _impactpoint) (`GameplayStatics.BreakHitResult` _outhit))
      (if _bblockinghit
        (set `self.StartAttached` true)
        (`SceneComponent.K2_SetWorldLocation` (`self.Cable`) _impactpoint false false)
        (else
          (set `self.StartAttached` false))))
    (:`then_1`
      (bind _outhit_2 (`KismetSystemLibrary.LineTraceSingle` _returnvalue_2 (+ _returnvalue_2 (* (`SceneComponent.GetForwardVector` _end) (`self.TraceDistance`)) (0.0 0.0 0.0)) "TraceTypeQuery1" false (`self.Out Actors`) "ForDuration" true (struct :`G` 0.989816 :`B` 1.0 :`A` 1.0) (struct :`G` 1.0 :`A` 1.0) 1.0))
      (bind (_bblockinghit_2 _binitialoverlap_2 _time_2 _distance_2 _location_2 _impactpoint_2) (`GameplayStatics.BreakHitResult` _outhit_2))
      (if _bblockinghit_2
        (set `self.EndAttached` true)
        (`SceneComponent.K2_SetWorldLocation` (`self.End`) _impactpoint_2 false false)
        (else
          (set `self.EndAttached` false))))
    (:`then_2`
      (bind _output_get_2 (set `CableComponent.CableLength` (* (+ _returnvalue_3 (/ _returnvalue_3 2.0)) (`self.CableLengthMult`)) (`self.Cable`)))
      (if (and (`self.StartAttached`) (`self.EndAttached`))
        (set `self.CanSpawn` true)
        (`SceneComponent.SetVisibility` (`self.Cable`) true true)
        (`self.SetActorHiddenInGame` false)
        (`MaterialInstanceDynamic.SetScalarParameterValue` (`self.DMI_Vines`) "TilingU" (/ _output_get_2 20.0))
        (else
          (set `self.CanSpawn` false)
          (`SceneComponent.SetVisibility` (`self.Cable`) true false)
          (`self.SetActorHiddenInGame` true))))))